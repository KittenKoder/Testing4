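; BP_TimeDriver is an actor that drives the time of day and moon phase of a referenced sky sphere.
; When automatic time is on, Tick advances a Day counter at a configurable speed, wrapping over a 30-day cycle.
; SetSky, also run at construction, derives day time from the fraction and moon phase from cycle position, flags full moon and eclipse windows, then updates the sky.
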(event EventBeginPlay)

(event Collision|EventActorBeginOverlap
  (params (OtherActor :type Actor%20Object%20Reference)))

(event EventTick
  (params (DeltaSeconds :type Float%20%28single-precision%29))
  (if (Variables|Controls|GetAutomaticTime)
    (bind _result (CallFunction|FloatWrap (+ (* DeltaSeconds (Variables|Controls|GetAutomaticDaySpeed)) (Variables|Controls|GetDay)) 3e+01))
    (Variables|Controls|SetDay _result)
    (CallFunction|SetSky)))

(fn ConstructionScript
  (CallFunction|SetSky))

(fn SetSky
  (bind _skysphere (Variables|Settings|GetSkySphere))
  (bind _day (Variables|Controls|GetDay))
  (bind _returnvalue (/ _day 3e+01))
  (Utilities|IsValid _skysphere
    (:Is%20Valid
      (Variables|/Game/Blueprints/Actors/BP_SkySphere.BP_SkySphere_C|SetDayTime _skysphere (Utilities|GetFraction _day))
      (Variables|/Game/Blueprints/Actors/BP_SkySphere.BP_SkySphere_C|SetMoonPhase _skysphere _returnvalue)
      (Variables|ReadOnly|SetIsFullMoon (and (> _returnvalue 0.49) (< _returnvalue 0.51)))
      (Variables|ReadOnly|SetIsEclipse (or (> _returnvalue 0.99) (< _returnvalue 0.01)))
      (Default|UpdateSky _skysphere))))